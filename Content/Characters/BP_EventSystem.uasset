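; Event system that triggers random breakdowns and ends the game when temperature maxes out.
; Tick shows the game-over widget and pauses at 100 temperature, otherwise uses a random-length Delay to pace RunEvent.
; RunEvent loops from a random index, firing the first pipe break or battery-box (minimap) event not already broken or cooling down.
; LowerTemp steps temperature down while enabled, switching itself off at zero.
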(event `LowerTemp`
  (if (<= (`self.TempAmount`) 0.0)
    (set `self.LowerTempOn` false)
    (elif (`self.LowerTempOn`)
      (set `self.TempAmount` (`KismetMathLibrary.FClamp` (- (`self.TempAmount`) 0.02) 0.0 100.0)))))

(event `self.ReceiveTick`
  (params (DeltaSeconds :type "Float (single-precision)"))
  (if (>= (`self.TempAmount`) 100.0)
    (bind _returnvalue (`|GenericCreateObject` "/Game/UI/WB_GameOver.WB_GameOver_C"))
    (`UserWidget.AddToViewport` _returnvalue 0)
    (set `PlayerController.bShowMouseCursor` false (`GameplayStatics.GetPlayerController` 0))
    (`GameplayStatics.SetGamePaused` true)
    (else
      (`KismetSystemLibrary.Delay` (`KismetMathLibrary.RandomFloatInRange` 6.0 8.0))
      (`self.RunEvent`))))

(event `RunEvent`
  (bind _maxevents (`self.MaxEvents`))
  ;[1 1 1] Look through available events
  (for _index (range (`KismetMathLibrary.RandomIntegerInRange` 0 _maxevents) (+ _maxevents 1)) :!label _label
    (`KismetSystemLibrary.PrintString` (`KismetStringLibrary.Conv_IntToString` _index))
    (switch `int` _index
      (:`1`
        ;[1 1 1] Pipe Break Event
        (bind _returnvalue (`GameplayStatics.GetActorOfClass` "/Game/Characters/BP_BrokenPipe.BP_BrokenPipe_C"))
        (cast `Actor` _returnvalue)
        (if (`/Game/Characters/BP_BrokenPipe.IsBroken` _returnvalue)
          _
          (elif (not (`/Game/Characters/BP_BrokenPipe.EventCooldown` _returnvalue))
            (`/Game/Characters/BP_BrokenPipe.EventPipeBreak` _returnvalue)
            (`self.BreakLoop`))))
      (:`2`
        ;[1 1 1] Minimap Break Event
        (bind _returnvalue_2 (`GameplayStatics.GetActorOfClass` "/Game/Characters/BP_BatteryBox.BP_BatteryBox_C"))
        (cast `Actor` _returnvalue_2)
        (if (`/Game/Characters/BP_BatteryBox.IsBroken` _returnvalue_2)
          _
          (elif (not (`/Game/Characters/BP_BatteryBox.EventCooldown` _returnvalue_2))
            (`/Game/Characters/BP_BatteryBox.EventNeedBatteries` _returnvalue_2)
            (`self.BreakLoop`)))))))

(event `BreakLoop`
  ;[1 1 1] Look through available events
  (goto _label :!via `Break`))

(fn `UserConstructionScript`)