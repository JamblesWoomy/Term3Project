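; BP_BrokenPipe is a repairable pipe prop that an event breaks and the player fixes through interaction.
; EventPipeBreak caches the tagged PlayerController and swaps in the broken mesh.
; While broken, overlap shows an outline overlay if the controller has the fix tool.
; Interact calls FixPipe, which, if broken, restores the fixed mesh, clears the player's "Item"-tagged mesh and sets a timed EventCooldown flag.
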(event `Cooldown`
  (set `self.EventCooldown` true)
  (`KismetSystemLibrary.Delay` 30.0)
  (set `self.EventCooldown` false))

(event `self.ReceiveBeginPlay`
  (set `self.EventCooldown` false))

(event `EventPipeBreak`
  ;[1 1 1] Set all starting variables
  (bind _outactors (`GameplayStatics.GetAllActorsWithTag` "PlayerController"))
  (set `self.PlayerController` (`|GetArrayItem` _outactors))
  (set `self.IsBroken` false)
  (`StaticMeshComponent.SetStaticMesh` (`self.Static Mesh`) "/Game/Models/Interior/Int_Drill_FullyBrokenPipe.Int_Drill_FullyBrokenPipe")
  (set `self.IsBroken` true))

(event `FixPipe`
  ;[1 1 1] Fixes the pipe when the player has the item
  (if (`self.IsBroken`)
    (`StaticMeshComponent.SetStaticMesh` (`self.Static Mesh`) "/Game/Assets/Interior/Int_Drill_FixedPipe.Int_Drill_FixedPipe")
    (for _array_element (`self.GetComponentsByTag` (`GameplayStatics.GetPlayerCharacter` 0) "/Script/Engine.StaticMeshComponent" "Item")
      _)
    (`StaticMeshComponent.SetStaticMesh` _array_element null)
    (set `self.IsBroken` false)
    (`self.Cooldown`)))

(event `self.ReceiveActorBeginOverlap`
  (params (OtherActor :type "Actor Object Reference"))
  ;[1 1 1] Display collision shader when broken
  (if (`self.IsBroken`)
    (bind _asfirst_person_controller (cast `/Game/Characters/FirstPersonController` (`self.PlayerController`)))
    (if (`/Game/Characters/FirstPersonController.HasFixTool` _asfirst_person_controller)
      (`MeshComponent.SetOverlayMaterial` (`self.Static Mesh`) "/Game/Materials/Outline_Mat_Inst.Outline_Mat_Inst"))))

(event `self.ReceiveActorEndOverlap`
  (params (OtherActor :type "Actor Object Reference"))
  ;[1 1 1] Display collision shader when broken
  (`MeshComponent.SetOverlayMaterial` (`self.Static Mesh`) null))

(fn `Interact`
  (returns (`Static Mesh` :type "StaticMesh Object Reference"))
  (`self.FixPipe`)
  (return (`StaticMeshComponent.StaticMesh` (`self.Static Mesh`))))

(fn `UserConstructionScript`)