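; Battery box actor with a door that opens and closes, showing an outline overlay on box and door while overlapped.
; SwitchDoorState toggles IsOpen and hides or restores the door mesh.
; Interact only flips IsOpen and returns the box's mesh, leaving the door visual untouched.
; BeginPlay caches BP_EventSystem, but the pipe-repair, temperature and cooldown-trigger logic that would use it is disconnected and never runs.
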(event `Cooldown`
  (set `self.EventCooldown` true)
  (`KismetSystemLibrary.Delay` 15.0)
  (set `self.EventCooldown` false))

(event `self.ReceiveBeginPlay`
  (set `self.EventCooldown` false)
  (bind _returnvalue (`GameplayStatics.GetActorOfClass` "/Game/Characters/BP_EventSystem.BP_EventSystem_C"))
  (set `self.EventSystem` _returnvalue))

(event `self.ReceiveActorBeginOverlap`
  (params (OtherActor :type "Actor Object Reference"))
  ;[1 1 1] Display collision shader
  (`MeshComponent.SetOverlayMaterial` (`self.Static Mesh`) "/Game/Materials/Outline_Mat_Inst.Outline_Mat_Inst")
  (`MeshComponent.SetOverlayMaterial` (`self.Door`) "/Game/Materials/Outline_Mat_Inst.Outline_Mat_Inst"))

(event `self.ReceiveActorEndOverlap`
  (params (OtherActor :type "Actor Object Reference"))
  ;[1 1 1] Display collision shader
  (`MeshComponent.SetOverlayMaterial` (`self.Static Mesh`) null)
  (`MeshComponent.SetOverlayMaterial` (`self.Door`) null))

(event `SwitchDoorState`
  (if (`self.IsOpen`)
    (set `self.IsOpen` false)
    (`StaticMeshComponent.SetStaticMesh` (`self.Door`) "/Game/Models/Interior/Int_Drill_BatteryDoor.Int_Drill_BatteryDoor")
    (else
      (set `self.IsOpen` true)
      (`StaticMeshComponent.SetStaticMesh` (`self.Door`) null))))

(fn `Interact`
  (returns (`Static Mesh` :type "StaticMesh Object Reference"))
  (if (`self.IsOpen`)
    (set `self.IsOpen` false)
    (else
      (set `self.IsOpen` true)))
  (return (`StaticMeshComponent.StaticMesh` (`self.Static Mesh`))))

(fn `UserConstructionScript`)