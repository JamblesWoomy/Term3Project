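; BP_Battery is an interactable box of battery meshes that the player picks up one at a time.
; Interact finds the battery component at BatteryIndex in a hard-coded array, decrements the index, returns that battery's static mesh and triggers its destruction after a short delay.
; Actor overlap toggles an outline overlay material on the box mesh.
; BeginPlay caches a FirstPersonController reference, which these graphs never use.
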(event `self.ReceiveBeginPlay`
  (bind _returnvalue (`GameplayStatics.GetActorOfClass` "/Game/Characters/FirstPersonController.FirstPersonController_C"))
  (set `self.CharREF` _returnvalue))

(event `Destroy Item`
  (params (ComponentErase :type "ActorComponent Object Reference"))
  ;[1 1 1] Erase the item gameobject and put it in the player's inventory
  (`KismetSystemLibrary.Delay` 0.2)
  (`ActorComponent.K2_DestroyComponent` ComponentErase))

(event `self.ReceiveActorBeginOverlap`
  (params (OtherActor :type "Actor Object Reference"))
  ;[1 1 1] Display collision shader
  (`MeshComponent.SetOverlayMaterial` (`self.BoxMesh`) "/Game/Materials/Outline_Mat_Inst.Outline_Mat_Inst"))

(event `self.ReceiveActorEndOverlap`
  (params (OtherActor :type "Actor Object Reference"))
  ;[1 1 1] Display collision shader
  (`MeshComponent.SetOverlayMaterial` (`self.BoxMesh`) null))

(fn `Interact`
  (returns (StaticMesh :type "StaticMesh Object Reference"))
  (`KismetSystemLibrary.PrintString` "Picked Up")
  (for (_array_element _array_index) (`|MakeArray` (`self.Battery1`) (`self.Battery2`) (`self.Battery3`) (`self.Battery4`) (`self.Battery5`) (`self.Battery6`) (`self.Battery7`) (`self.Battery8`) (`self.Battery9`) (`self.Battery10`) (`self.Battery11`) (`self.Battery12`) (`self.Battery13`) (`self.Battery14`) (`self.Battery15`) (`self.Battery16`) (`self.Battery18`))
    (if (== _array_index (`self.BatteryIndex`))
      (`self.Destroy Item` _array_element)
      (set `self.BatteryIndex` (- (`self.BatteryIndex`) 1))
      (return (`StaticMeshComponent.StaticMesh` _array_element)))))

(fn `UserConstructionScript`)