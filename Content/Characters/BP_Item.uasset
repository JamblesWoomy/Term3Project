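; BP_Item is a pickup item actor that highlights on overlap and removes itself when interacted with.
; Overlap begin and end set and clear an outline overlay material on its static mesh, without filtering the overlapping actor.
; Interact prints a pickup message, triggers DestroyItem and returns the mesh asset to the caller.
; DestroyItem waits briefly before destroying the actor.
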(event `Destroy Item`
  (`KismetSystemLibrary.Delay` 0.2)
  (`self.K2_DestroyActor`))

(event `self.ReceiveActorBeginOverlap`
  (params (OtherActor :type "Actor Object Reference"))
  (`MeshComponent.SetOverlayMaterial` (`self.Static Mesh`) "/Game/Materials/Outline_Mat_Inst.Outline_Mat_Inst"))

(event `self.ReceiveActorEndOverlap`
  (params (OtherActor :type "Actor Object Reference"))
  (`MeshComponent.SetOverlayMaterial` (`self.Static Mesh`) null))

(fn `Interact`
  (returns (`Static Mesh` :type "StaticMesh Object Reference"))
  (`KismetSystemLibrary.PrintString` "Picked Up")
  (`self.Destroy Item`)
  (return (`StaticMeshComponent.StaticMesh` (`self.Static Mesh`))))

(fn `UserConstructionScript`)