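; Ladder actor that teleports the first-person player between two ends instead of animating a climb.
; LadderWarp shows a fade-to-black widget, waits briefly, then moves the last overlapping player to one of two stored points, toggling UpDown each use.
; Point locations are relative to the ladder, while rotations apply unconverted.
; Overlap toggles an outline overlay material on the mesh; Interact is empty here.
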(event `LadderWarp`
  (bind (_tp_pos_location _tp_pos_rotation) (`KismetMathLibrary.BreakTransform` (`self.TP_Pos`)))
  (bind (_tp_oldpos_location _tp_oldpos_rotation) (`KismetMathLibrary.BreakTransform` (`self.TP_OldPos`)))
  (bind _returnvalue (`|CreateWidget` "/Game/FadeToBlackBlueprint.FadeToBlackBlueprint_C"))
  (`UserWidget.AddToViewport` _returnvalue 0)
  (`KismetSystemLibrary.Delay` 0.25)
  (bind _asfirst_person_movement (cast `/Game/Characters/FirstPersonMovement` (stale `self.ReceiveActorBeginOverlap` OtherActor)))
  (if (`self.UpDown`)
    (`self.K2_SetActorLocationAndRotation` _asfirst_person_movement (`KismetMathLibrary.TransformLocation` (`self.GetTransform`) _tp_oldpos_location) _tp_oldpos_rotation false false)
    (set `self.UpDown` false)
    (else
      (`self.K2_SetActorLocationAndRotation` _asfirst_person_movement (`KismetMathLibrary.TransformLocation` (`self.GetTransform`) _tp_pos_location) _tp_pos_rotation false false)
      (set `self.UpDown` true))))

(event `self.ReceiveActorBeginOverlap`
  (params (OtherActor :type "Actor Object Reference"))
  ;[1 1 1] Display collision shader
  (`MeshComponent.SetOverlayMaterial` (`self.Static Mesh`) "/Game/Materials/Outline_Mat_Inst.Outline_Mat_Inst"))

(event `self.ReceiveActorEndOverlap`
  (params (OtherActor :type "Actor Object Reference"))
  ;[1 1 1] Display collision shader
  (`MeshComponent.SetOverlayMaterial` (`self.Static Mesh`) null))

(fn `Interact`
  (returns (`Static Mesh` :type "StaticMesh Object Reference")))

(fn `UserConstructionScript`)