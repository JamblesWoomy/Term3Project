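; BP_TapeItem is a pickup holding eight tape meshes that are taken one at a time.
; Overlap applies an outline overlay material to the box mesh and clears it when the overlap ends.
; Interact selects the tape at TapeIndex, starts its delayed component destruction, advances the index and returns its static mesh to the caller.
; BeginPlay caches the FirstPersonController actor, though the visible logic never uses it.
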(event `self.ReceiveBeginPlay`
  (bind _returnvalue (`GameplayStatics.GetActorOfClass` "/Game/Characters/FirstPersonController.FirstPersonController_C"))
  (set `self.CharREF` _returnvalue))

(event `self.ReceiveActorBeginOverlap`
  (params (OtherActor :type "Actor Object Reference"))
  ;[1 1 1] Display collision shader
  (`MeshComponent.SetOverlayMaterial` (`self.BoxMesh`) "/Game/Materials/Outline_Mat_Inst.Outline_Mat_Inst"))

(event `self.ReceiveActorEndOverlap`
  (params (OtherActor :type "Actor Object Reference"))
  ;[1 1 1] Display collision shader
  (`MeshComponent.SetOverlayMaterial` (`self.BoxMesh`) null))

(event `Destroy Item`
  (params (NewParam :type "ActorComponent Object Reference"))
  ;[1 1 1] Erase the item gameobject and put it in the player's inventory
  (`KismetSystemLibrary.Delay` 0.2)
  (`ActorComponent.K2_DestroyComponent` NewParam))

(fn `Interact`
  (returns (StaticMesh :type "StaticMesh Object Reference"))
  (`KismetSystemLibrary.PrintString` "Picked Up")
  (for (_array_element _array_index) (`|MakeArray` (`self.Tape1`) (`self.Tape2`) (`self.Tape3`) (`self.Tape4`) (`self.Tape5`) (`self.Tape6`) (`self.Tape7`) (`self.Tape8`))
    (if (== _array_index (`self.TapeIndex`))
      (`self.Destroy Item` _array_element)
      (set `self.TapeIndex` (+ (`self.TapeIndex`) 1))
      (return (`StaticMeshComponent.StaticMesh` _array_element)))))

(fn `UserConstructionScript`)