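; BP_NavButtonForward is the forward navigation lever that pushes the MinimapDrill along its forward vector.
; MoveDrill offsets the drill, raises BP_EventSystem's clamped temperature and plays the lever animation once, as neither state flag resets here.
; Tick calls LowerTemp on the event system unconditionally.
; Actor overlap toggles an outline overlay material, and the Interact function is an empty stub.
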(event `self.ReceiveTick`
  (params (DeltaSeconds :type "Float (single-precision)"))
  ;[1 1 1] Lower temperature when not using  lever
  (`/Game/Characters/BP_EventSystem.LowerTemp` (`self.EventSystem`)))

(event `PlayAnim`
  (bind _skeletalmesh (`self.SkeletalMesh`))
  ;[1 1 1] Play animation for lever pull
  (if (`self.RunningDrill`)
    (if (not (`self.AnimationRun`))
      (`SkeletalMeshComponent.PlayAnimation` _skeletalmesh "/Game/Animations/LeverPullMain/AnimMainLever_Anim.AnimMainLever_Anim" false)
      (`KismetSystemLibrary.PrintString` "Hello"))
    (else
      (`SkeletalMeshComponent.PlayAnimation` _skeletalmesh "/Game/Animations/LeverPullMain/AnimMainLever_AnimReverse.AnimMainLever_AnimReverse" false)
      (`SkeletalMeshComponent.SetPosition` _skeletalmesh 0.583333 true))))

(event `self.ReceiveBeginPlay`
  ;[1 1 1] Get Event System
  (bind _returnvalue (`GameplayStatics.GetActorOfClass` "/Game/Characters/BP_EventSystem.BP_EventSystem_C"))
  (set `self.EventSystem` _returnvalue))

(event `MoveDrill`
  ;[1 1 1] Push the Minimap drill by its forward vector
  (set `self.RunningDrill` true)
  (bind _returnvalue (`GameplayStatics.GetActorOfClass` "/Game/Assets/DrillMap/MinimapDrill.MinimapDrill_C"))
  (`self.K2_SetActorLocation` _returnvalue (+ (`self.K2_GetActorLocation` _returnvalue) (* (`self.GetActorForwardVector` _returnvalue) 8.0)) false false)
  (set `/Game/Characters/BP_EventSystem.TempAmount` (`KismetMathLibrary.FClamp` (+ (`/Game/Characters/BP_EventSystem.TempAmount` (`self.EventSystem`)) 0.05) 0.0 100.0) (`self.EventSystem`))
  (`self.PlayAnim`)
  (set `self.AnimationRun` true))

(event `self.ReceiveActorBeginOverlap`
  (params (OtherActor :type "Actor Object Reference"))
  ;[1 1 1] Display collision shader
  (`MeshComponent.SetOverlayMaterial` (`self.SkeletalMesh`) "/Game/Materials/Outline_Mat_Inst.Outline_Mat_Inst"))

(event `self.ReceiveActorEndOverlap`
  (params (OtherActor :type "Actor Object Reference"))
  ;[1 1 1] Display collision shader
  (`MeshComponent.SetOverlayMaterial` (`self.SkeletalMesh`) null))

(fn `Interact`
  (returns (StaticMesh :type "StaticMesh Object Reference"))
  (return null))

(fn `UserConstructionScript`)